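; Base actor for destructible objects that lose health while hit by a laser and destroy themselves when it runs out.
; LaserHit applies a faded white overlay once through a DoOnce, decrements and prints Health, then checks for destruction.
; LaserHitEnd clears the overlay and re-arms the DoOnce.
; A temporary helper reflects a laser vector off an impact normal and debug-traces it, leaving the result unused.
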(event `OverlayMaterialReset`
  (goto _label :!via `Reset`))

(event `/Game/Blueprints/Interfaces/BPI_LaserTrace.LaserHit`
  (`|ExecutionSequence`
    (:`then_0`
      (`/Engine/EditorBlueprintResources/StandardMacros.DoOnce` false :!label _label
        (:`Completed`
          (`MeshComponent.SetOverlayMaterial` (`self.StaticMesh`) "/Game/LevelPrototyping/Materials/MI_FadedWhite.MI_FadedWhite"))))
    (:`then_1`
      (bind _result (`/Engine/EditorBlueprintResources/StandardMacros.DecrementFloat` (`self.Health`))
        (:`  `
          (`KismetSystemLibrary.PrintString` (`KismetStringLibrary.Conv_DoubleToString` _result))
          (if (<= (`self.Health`) 0.0)
            (`self.K2_DestroyActor`)))))))

(event `/Game/Blueprints/Interfaces/BPI_LaserTrace.LaserHitEnd`
  (`MeshComponent.SetOverlayMaterial` (`self.StaticMesh`) null)
  (`self.OverlayMaterialReset`))

(fn `(Temperory)MirroredLaserTrace`
  (params (ImpactNormal :type "Vector Structure") (Location :type "Vector Structure") (TraceEnd :type "Vector Structure") (TraceStart :type "Vector Structure"))
  (locals (IncidentVector :type "Vector Structure") (ReflectedVector :type "Vector Structure"))
  (set `local.IncidentVector` (- TraceEnd TraceStart))
  (bind _output_get (set `local.ReflectedVector` (- (`local.IncidentVector`) (* (* (`KismetMathLibrary.Dot_VectorVector` (`local.IncidentVector`) ImpactNormal) ImpactNormal) 2.0))))
  (bind _outhit (`KismetSystemLibrary.LineTraceSingle` :`Start` Location :`End` (* _output_get 1000.0) :`TraceChannel` "TraceTypeQuery1" :`DrawDebugType` "ForOneFrame" :`TraceColor` (struct :`G` 0.913099 :`B` 1.0 :`A` 1.0) :`TraceHitColor` (struct :`G` 0.913099 :`B` 1.0 :`A` 1.0))))

(fn `UserConstructionScript`)