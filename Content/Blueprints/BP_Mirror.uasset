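; BP_Mirror is a mirror that reflects an incoming laser by spawning and steering its own BP_Laser.
; MirrorLaser computes the reflection vector from trace direction and impact normal, spawns the laser through a DoOnce, and moves it to the hit location each call.
; Its rotation looks at the scaled reflection vector, used as a world-space point.
; LaserHitEnd destroys the laser and resets the DoOnce.
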(event `LaserSpawnerReset`
  (goto _label :!via `Reset`))

(event `/Game/Blueprints/Interfaces/BPI_LaserTrace.MirrorLaser`
  (params (ImpactNormal :type "Vector Structure") (Location :type "Vector Structure") (TraceEnd :type "Vector Structure") (TraceStart :type "Vector Structure"))
  (`self.MirrorTrace` ImpactNormal TraceEnd TraceStart)
  (`|ExecutionSequence`
    (:`then_0`
      (`/Engine/EditorBlueprintResources/StandardMacros.DoOnce` false :!label _label
        (:`Completed`
          (bind _returnvalue (`|SpawnActorFromClass` "/Game/Blueprints/BP_Laser.BP_Laser_C" (`KismetMathLibrary.MakeTransform` Location) "Undefined" "MultiplyWithRoot" null (`|MakeArray` self (`GameplayStatics.GetPlayerCharacter` 0) :!type "Actor Object Reference") 1000.0 null))
          (set `self.Laser` _returnvalue))))
    (:`then_1`
      (`self.K2_SetActorLocation` (`self.Laser`) Location false false)
      (`self.K2_SetActorRotation` (`self.Laser`) (`KismetMathLibrary.FindLookAtRotation` Location (* (`self.ReflectedVectorr`) 1000.0)) false))))

(event `/Game/Blueprints/Interfaces/BPI_LaserTrace.LaserHitEnd`
  (`self.K2_DestroyActor` (`self.Laser`))
  (`self.LaserSpawnerReset`))

(fn `UserConstructionScript`)