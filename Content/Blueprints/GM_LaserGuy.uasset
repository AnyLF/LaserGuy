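; GM_LaserGuy is a game mode Blueprint that sets up the camera canvas UI and supplies camera data.
; On BeginPlay it adds the WBP_CameraCanvas widget to the viewport and resets LaserStabilization, whose increment logic is unconnected.
; Getter functions return the CameraLocation actor's transform and location as pivot and camera target, plus a fixed camera parameter.
; RestartLevel reloads the current level by name.
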(event `self.ReceiveTick`
  (params (DeltaSeconds :type "Float (single-precision)"))
  ;[1 1 1] asd
)

(event `self.ReceiveBeginPlay`
  (`KismetSystemLibrary.PrintString` "GM STARTED")
  (bind _returnvalue (`|CreateWidget` "/Game/Blueprints/UGM/WBP_CameraCanvas.WBP_CameraCanvas_C"))
  (`UserWidget.AddToViewport` _returnvalue 0)
  (set `self.LaserStabilization` 0.0))

(fn `Get_3P_PivotTarget`
  (returns (ReturnValue :type "Transform Structure"))
  (return (`self.GetTransform` (`self.CameraLocation`))))

(fn `Get_CameraParameters`
  (returns (FP_FOV :type "Float (double-precision)"))
  (return 90.0))

(fn `Get_CameraTarget`
  (returns (ReturnValue :type "Vector Structure"))
  (return (`self.K2_GetActorLocation` (`self.CameraLocation`))))

(fn `RestartLevel`
  (bind _returnvalue (`GameplayStatics.GetCurrentLevelName` true))
  (`GameplayStatics.OpenLevel` (`KismetStringLibrary.Conv_StringToName` _returnvalue)))

(fn `UserConstructionScript`)