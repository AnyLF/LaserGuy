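; Player controller for the LaserGuy character that makes the pawn aim at the mouse cursor.
; On BeginPlay it registers the default Enhanced Input mapping context with the local player subsystem.
; Each Tick it traces under the cursor on the Visibility channel and passes the point to player character 0 through LookAtMessage.
; The point's X is shifted by the height gap between slightly above the character's origin and the hit.
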(event `self.ReceiveBeginPlay`
  (bind _returnvalue (subsystem `EnhancedInputLocalPlayerSubsystem`))
  ;[0.01042 0.01042 0.01042] Add Mapping Context
  (`/Engine/EditorBlueprintResources/StandardMacros.IsValid` _returnvalue
    (:`Is Valid`
      (`EnhancedInputSubsystemInterface.AddMappingContext` _returnvalue "/Game/Blueprints/Input/IMC_Default.IMC_Default" 0 (struct)))))

(event `self.ReceiveTick`
  (params (DeltaSeconds :type "Float (single-precision)"))
  (bind (_bblockinghit _binitialoverlap _time _distance _location) (`GameplayStatics.BreakHitResult` (`self.GetHitResultUnderCursorByChannel` "TraceTypeQuery1" false)))
  (bind (_returnvalue_x _returnvalue_y _returnvalue_z) (`KismetMathLibrary.BreakVector` (`self.K2_GetActorLocation` (`GameplayStatics.GetPlayerCharacter` 0))))
  (message `/Game/Blueprints/Interfaces/BPI_LaserGuy.LookAt` (`GameplayStatics.GetPlayerCharacter` 0) (`KismetMathLibrary.MakeVector` (- (.x _location) (- (+ _returnvalue_z 25.0) (.z _location))) (.y _location) (.z _location))))

(fn `UserConstructionScript`)