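; Player controller for the LaserGuy character, prefixed OLD, that handles input setup, camera possession and cursor aiming.
; On BeginPlay it adds the default Enhanced Input mapping context, and on possessing a pawn it passes that pawn to BP_CameraManager's OnPossess.
; Every tick it traces under the mouse cursor and sends the hit location to player character 0 through LookAtMessage.
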(event `self.ReceiveBeginPlay`
  (bind _returnvalue (subsystem `EnhancedInputLocalPlayerSubsystem`))
  ;[0.01042 0.01042 0.01042] Add Mapping Context
  (`/Engine/EditorBlueprintResources/StandardMacros.IsValid` _returnvalue
    (:`Is Valid`
      (`EnhancedInputSubsystemInterface.AddMappingContext` _returnvalue "/Game/Blueprints/Input/IMC_Default.IMC_Default" 0 (struct)))))

(event `self.ReceivePossess`
  (params (PossessedPawn :type "Pawn Object Reference"))
  ;[0.02083 0.02083 0.02083] Call "OnPossess" in Camera Manager when possessing the pawn
  (bind _asbp_camera_manager (cast `/Game/Blueprints/CameraSystem/BP_CameraManager` (`self.PlayerCameraManager`)))
  (`/Game/Blueprints/CameraSystem/BP_CameraManager.OnPossess` _asbp_camera_manager PossessedPawn))

(event `self.ReceiveTick`
  (params (DeltaSeconds :type "Float (single-precision)"))
  (message `/Game/Blueprints/Interfaces/BPI_LaserGuy.LookAt` (`GameplayStatics.GetPlayerCharacter` 0) (`.Location` (`GameplayStatics.BreakHitResult` (`self.GetHitResultUnderCursorByChannel` "TraceTypeQuery3" false)))))

(fn `UserConstructionScript`)