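; BP_Laser is a laser beam actor that sphere-traces forward each tick, sizing its beam and placing an impact effect at the hit.
; It sends hit, mirror and hit-end messages to traced actors as contact changes.
; ReflectSelf computes a reflection vector and spawns one reusable child BP_Laser at the impact, forming chains that DestroyReflectedLaser removes recursively.
; Freeze and UnFreeze toggle visibility and gate the trace.
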(event `self.ReceiveTick`
  (params (DeltaSeconds :type "Float (single-precision)"))
  (bind _returnvalue (`self.K2_GetActorLocation`))
  (`/Engine/EditorBlueprintResources/StandardMacros.Gate` false :!label _label
    (:`Exit`
      (bind (_outhit _returnvalue_2) (`KismetSystemLibrary.SphereTraceSingle` _returnvalue (+ _returnvalue (* (`self.GetActorForwardVector`) (`self.Distance`))) 15.0 "TraceTypeQuery1" false (`self.IgnoreActors`)))
      (set `self.isHit?` _returnvalue_2)
      (bind (_bblockinghit _binitialoverlap _time _distance _location _impactpoint _normal _impactnormal _physmat _hitactor _hitcomponent _hitbonename _bonename _hititem _elementindex _faceindex _tracestart _traceend) (`GameplayStatics.BreakHitResult` _outhit))
      (`FXSystemComponent.SetVectorParameter` (`self.Laser`) "Beam End" (select `bool` (`self.isHit?`) :`false` (`KismetMathLibrary.MakeVector` (`self.Distance`)) :`true` (`KismetMathLibrary.MakeVector` _distance) :!type "Vector Structure"))
      (`SceneComponent.SetVisibility` (`self.LaserImpact`) (`self.isHit?`) false)
      (if (`self.isHit?`)
        (`SceneComponent.K2_SetWorldLocation` (`self.LaserImpact`) _location false false)
        (`self.Actor`
          (:`then`
            (if (== (`self.Actor`) _hitactor)
              (message `/Game/Blueprints/Interfaces/BPI_LaserTrace.LaserHit` _hitactor :!label _label_2)
              (message `/Game/Blueprints/Interfaces/BPI_LaserTrace.MirrorLaser` _hitactor _impactnormal _location _traceend _tracestart self)
              (else
                (message `/Game/Blueprints/Interfaces/BPI_LaserTrace.LaserHitEnd` (`self.Actor`) self :!label _label_3))))
          (:`else`
            (set `self.Actor` _hitactor)
            (goto _label_2)))
        (else
          (goto _label_3)))
      (set `self.Actor` _hitactor))))

(event `UnFreeze`
  (`SceneComponent.SetVisibility` (`self.LaserImpact`) true false)
  (`SceneComponent.SetVisibility` (`self.Laser`) true false)
  (goto _label :!via `Open`))

(event `Freeze`
  (`SceneComponent.SetVisibility` (`self.Laser`) false false)
  (`SceneComponent.SetVisibility` (`self.LaserImpact`) false false)
  (goto _label :!via `Close`))

(event `SpawnReflectedLaser`
  (params (`[0]` :type "Actor Object Reference"))
  (`/Engine/EditorBlueprintResources/StandardMacros.DoOnce` false :!label _label_4
    (:`Completed`
      (bind _returnvalue (`|SpawnActorFromClass` "BP_Laser_C" (`KismetMathLibrary.MakeTransform` (0.0 0.0 0.0)) "Undefined" "MultiplyWithRoot" null (`|MakeArray` `[0]` (`GameplayStatics.GetPlayerCharacter` 0) :!type "Actor Object Reference") 3000.0 null))
      (set `self.ReflectedLaser` _returnvalue))))

(event `ResetSpawnReflectedLaser`
  (goto _label_4 :!via `Reset`))

(fn `DestroyReflectedLaser`
  (bind _reflectedlaser (`self.ReflectedLaser`)
    (:`then`
      (`self.DestroyReflectedLaser` _reflectedlaser)
      (`self.K2_DestroyActor` _reflectedlaser)
      (set `self.ReflectedLaser` null)
      (`self.ResetSpawnReflectedLaser`))
    (:`else`)))

(fn `ReflectSelf`
  (params (ImplactNormal :type "Vector Structure") (Location :type "Vector Structure") (TraceEnd :type "Vector Structure") (TraceStart :type "Vector Structure") (Mirror :type "/Game/Blueprints/Objects/BP_Mirror Object Reference"))
  (locals (IncidentVector :type "Vector Structure") (ReflectedVector :type "Vector Structure"))
  (set `local.IncidentVector` (- TraceEnd TraceStart))
  (set `local.ReflectedVector` (- (`local.IncidentVector`) (* (* (`KismetMathLibrary.Dot_VectorVector` (`local.IncidentVector`) ImplactNormal) ImplactNormal) 2.0)))
  (`|ExecutionSequence`
    (:`then_0`
      (`self.SpawnReflectedLaser` Mirror))
    (:`then_1`
      (`self.K2_SetActorLocation` (`self.ReflectedLaser`) Location false false)
      (`self.K2_SetActorRotation` (`self.ReflectedLaser`) (`KismetMathLibrary.FindLookAtRotation` Location (* (`local.ReflectedVector`) 1000.0)) false))))

(fn `UserConstructionScript`)