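; BP_NPC_Movable is an NPC that walks a repeating patrol route through an array of destination actors.
; On BeginPlay it sets its walk speed from Speed, then calls AI MoveTo toward the current destination's location.
; Each success advances the index, wraps at the end, and loops back after a tiny Delay.
; A failed move is not handled, so the patrol stops there.
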(event `self.ReceiveBeginPlay`
  (`parent.ReceiveBeginPlay`)
  (set `CharacterMovementComponent.MaxWalkSpeed` (`self.Speed`) (`self.CharacterMovement`))
  (`|AIMoveTo` self (`self.K2_GetActorLocation` (`|GetArrayItem` (`self.Destination`) (`self.Index`))) null :!label _label
    (:`OnSuccess`
      (bind _result (`/Engine/EditorBlueprintResources/StandardMacros.IncrementInt` (`self.Index`))
        (:`  `
          (if (>= _result (`KismetArrayLibrary.Array_Length` (`self.Destination`)))
            (set `self.Index` 0))
          (`KismetSystemLibrary.Delay` 0.001)
          (goto _label))))))

(fn `UserConstructionScript`
  (`parent.UserConstructionScript`))