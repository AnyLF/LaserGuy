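; BP_NPC_Base is an NPC base Blueprint for the LaserGuy game that restarts the level when hit by a laser.
; BeginPlay caches the player and game mode, then randomizes the body and head meshes.
; Pawn sensing latches a flag on first sighting the player, after which Tick turns the head on yaw only to track them.
; LaserHit calls the game mode's RestartLevel through a DoOnce guard.
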(event `self.ReceiveBeginPlay`
  (bind _asbp_laser_guy (cast `/Game/Blueprints/BP_LaserGuy` (`GameplayStatics.GetPlayerCharacter` 0)))
  (set `self.As BP Laser Guy` _asbp_laser_guy)
  (bind _asgm_laser_guy (cast `/Game/Blueprints/GM_LaserGuy` (`GameplayStatics.GetGameMode`)))
  (set `self.As GM Laser Guy` _asgm_laser_guy)
  (`StaticMeshComponent.SetStaticMesh` (`self.Body`) (select `int` (`KismetMathLibrary.RandomIntegerInRange` 0 3) :`0` "/Game/LevelPrototyping/Meshes/LaserGuy/NPC/NPC_Body_NPC_1.NPC_Body_NPC_1" :`1` "/Game/LevelPrototyping/Meshes/LaserGuy/NPC/NPC_Body_NPC_2.NPC_Body_NPC_2" :`2` "/Game/LevelPrototyping/Meshes/LaserGuy/NPC/NPC_Body_NPC_3.NPC_Body_NPC_3" :`3` "/Game/LevelPrototyping/Meshes/LaserGuy/NPC/NPC_Body_NPC_4.NPC_Body_NPC_4" :!type "StaticMesh Object Reference"))
  (`StaticMeshComponent.SetStaticMesh` (`self.Head`) (select `int` (`KismetMathLibrary.RandomIntegerInRange` 0 9) :`0` "/Game/LevelPrototyping/Meshes/LaserGuy/LaserGuy_Head_Sphere_Red.LaserGuy_Head_Sphere_Red" :`1` "/Game/LevelPrototyping/Meshes/LaserGuy/LaserGuy_Head_Sphere_Blue.LaserGuy_Head_Sphere_Blue" :`2` "/Game/LevelPrototyping/Meshes/LaserGuy/LaserGuy_Head_Sphere_Green.LaserGuy_Head_Sphere_Green" :`3` "/Game/LevelPrototyping/Meshes/LaserGuy/LaserGuy_Head_Sphere_Pink.LaserGuy_Head_Sphere_Pink" :`4` "/Game/LevelPrototyping/Meshes/LaserGuy/LaserGuy_Head_Sphere_Yellow.LaserGuy_Head_Sphere_Yellow" :`5` "/Game/LevelPrototyping/Meshes/LaserGuy/LaserGuy_Body_Cube_Red.LaserGuy_Body_Cube_Red" :`6` "/Game/LevelPrototyping/Meshes/LaserGuy/LaserGuy_Body_Cube_Blue.LaserGuy_Body_Cube_Blue" :`7` "/Game/LevelPrototyping/Meshes/LaserGuy/LaserGuy_Body_Cube_Green.LaserGuy_Body_Cube_Green" :`8` "/Game/LevelPrototyping/Meshes/LaserGuy/LaserGuy_Body_Cube_Pink.LaserGuy_Body_Cube_Pink" :`9` "/Game/LevelPrototyping/Meshes/LaserGuy/LaserGuy_Body_Cube_Yellow.LaserGuy_Body_Cube_Yellow" :!type "StaticMesh Object Reference")))

(event `/Game/Blueprints/Interfaces/BPI_LaserTrace.LaserHit`
  (`/Engine/EditorBlueprintResources/StandardMacros.DoOnce` false
    (:`Completed`
      (`GameModeLaserGuy.RestartLevel` (`self.As GM Laser Guy`)))))

(event `self.PawnSensing.OnSeePawn`
  (params (Pawn :type "Pawn Object Reference"))
  (cast `/Game/Blueprints/BP_LaserGuy` Pawn)
  (set `self.CanSeePlayer` true))

(event `self.ReceiveTick`
  (params (DeltaSeconds :type "Float (single-precision)"))
  (bind _head (`self.Head`))
  (bind (_returnvalue_roll _returnvalue_pitch _returnvalue_yaw) (`KismetMathLibrary.BreakRotator` (`KismetMathLibrary.FindLookAtRotation` (`SceneComponent.K2_GetComponentLocation` _head) (`self.K2_GetActorLocation` (`self.As BP Laser Guy`)))))
  (if (`self.CanSeePlayer`)
    (`SceneComponent.K2_SetWorldRotation` _head (`KismetMathLibrary.MakeRotator` 0.0 0.0 _returnvalue_yaw) false false)))

(fn `UserConstructionScript`
  (`parent.UserConstructionScript`))