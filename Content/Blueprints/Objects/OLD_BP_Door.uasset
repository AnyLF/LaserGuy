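; Door actor, prefixed OLD, that slides its Door component open and closed through OpenDoor and CloseDoor events.
; Each direction has its own timeline driving an ease-in of relative location, toward DoorMoveLocation or back to zero, and stops the opposing timeline first.
; Each update eases from the door's current location rather than a stored start.
; A DoOnce blocks repeated opens until CloseDoor resets it.
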(event `OpenDoor`
  (bind _door (`self.Door`))
  (bind _door_2 (`self.Door`))
  (`/Engine/EditorBlueprintResources/StandardMacros.DoOnce` false :!label _label
    (:`Completed`
      (`|ExecutionSequence`
        (:`then_0`
          (bind (_direction _alpha) (`Timeline|Timeline_0` :!via `Stop` :!label _label_2)
            (:`Update`
              (`SceneComponent.K2_SetRelativeLocation` _door (`|EaseFunction` "EaseIn" _alpha (`SceneComponent.RelativeLocation` _door)) false false))))
        (:`then_1`
          (bind (_direction_2 _alpha_2) (`Timeline|Timeline` :!via `PlayFromStart` :!label _label_3)
            (:`Update`
              (`SceneComponent.K2_SetRelativeLocation` _door_2 (`|EaseFunction` "EaseIn" _alpha_2 (`SceneComponent.RelativeLocation` _door_2) (`self.DoorMoveLocation`)) false false))))))))

(event `CloseDoor`
  (`|ExecutionSequence`
    (:`then_0`
      (goto _label_3 :!via `Stop`))
    (:`then_1`
      (goto _label_2 :!via `PlayFromStart`))
    (:`then_2`
      (goto _label :!via `Reset`))))

(fn `UserConstructionScript`)