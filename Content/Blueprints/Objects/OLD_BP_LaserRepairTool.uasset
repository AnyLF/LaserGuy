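; An older laser repair tool pickup that, on overlap with BP_LaserGuy, lowers LaserStabilization in GM_LaserGuy by a fixed amount, clamped at zero, then destroys itself.
; While idle, its sphere bobs vertically on a timeline.
; The idle event starts on BeginPlay and re-calls itself when the timeline finishes, using a FlipFlop to alternate forward and reverse playback.
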(event `IdleAnimation`
  ;[1 1 1] Idle Animation
  (`/Engine/EditorBlueprintResources/StandardMacros.FlipFlop`
    (:`A`
      (bind (_direction _z_25_to_100) (`Timeline|İdle` :!via `PlayFromStart` :!label _label)
        (:`Update`
          (`SceneComponent.K2_SetRelativeLocation` (`self.Sphere`) (`KismetMathLibrary.MakeVector` 0.0 0.0 _z_25_to_100) false false))
        (:`Finished`
          (`self.IdleAnimation`))))
    (:`B`
      (goto _label :!via `ReverseFromEnd`))))

(event `self.ReceiveBeginPlay`
  (`self.IdleAnimation`))

(event `self.ReceiveActorBeginOverlap`
  (params (OtherActor :type "Actor Object Reference"))
  (cast `/Game/Blueprints/BP_LaserGuy` OtherActor)
  (bind _asgm_laser_guy (cast `/Game/Blueprints/GM_LaserGuy` (`GameplayStatics.GetGameMode`)))
  (set `GameModeLaserGuy.LaserStabilization` (`KismetMathLibrary.FMax` (- (`GameModeLaserGuy.LaserStabilization` _asgm_laser_guy) 25.0)) _asgm_laser_guy)
  (`self.K2_DestroyActor`))

(fn `UserConstructionScript`)