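; BP_FrozenBarrel is a destructible barrel child Blueprint that freezes nearby actors when destroyed.
; Its DestroyObject override spawns two Niagara effects at the mesh, then runs a multi sphere trace on the Visibility channel around the actor.
; Each hit actor receives a Freeze interface message with FreezeDuration, so targets handle their own response, before the parent's destroy logic runs.
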(event `self.DestroyObject`
  (bind _returnvalue (`self.K2_GetActorLocation`))
  (bind _returnvalue_2 (`SceneComponent.K2_GetComponentLocation` (`self.StaticMesh`)))
  (`NiagaraFunctionLibrary.SpawnSystemAtLocation` "/Game/sA_Megapack_v1/sA_SkillSet_1/Fx/NiagaraSystems/NS_Thorn_3.NS_Thorn_3" _returnvalue_2)
  (`NiagaraFunctionLibrary.SpawnSystemAtLocation` "/Game/sA_Megapack_v1/sA_SkillSet_1/Fx/NiagaraSystems/NS_Hit_Ray.NS_Hit_Ray" _returnvalue_2)
  (bind _outhits (`KismetSystemLibrary.SphereTraceMulti` :`Start` _returnvalue :`End` _returnvalue :`Radius` 240.0 :`TraceChannel` "TraceTypeQuery1" :`TraceColor` (struct :`G` 0.933595 :`B` 1.0 :`A` 1.0) :`TraceHitColor` (struct :`G` 0.208508 :`B` 1.0 :`A` 1.0) :`DrawTime` 3.0))
  (for _array_element _outhits
    (message `/Game/Blueprints/Interfaces/BPI_LaserGuy.Freeze` (`.HitActor` (`GameplayStatics.BreakHitResult` _array_element)) (`self.Freeze Duration`)))
  (`parent.DestroyObject`))

(fn `UserConstructionScript`
  (`parent.UserConstructionScript`))