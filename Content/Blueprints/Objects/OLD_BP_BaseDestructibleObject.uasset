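; Legacy base destructible object that loses health while hit by a laser and destroys itself at zero.
; LaserHit applies a faded white overlay material through a DoOnce gate and decrements Health on every call.
; LaserHitEnd clears the overlay and resets the gate for the next hit.
; A temporary, uncalled helper debug-traces a reflected laser ray from an impact normal, leaving the result unused.
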(event `ResetDamageEffect`
  (goto _label :!via `Reset`))

(event `/Game/Blueprints/Interfaces/BPI_LaserTrace.LaserHit`
  (`|ExecutionSequence`
    (:`then_0`
      (`/Engine/EditorBlueprintResources/StandardMacros.DoOnce` false :!label _label
        (:`Completed`
          (`self.DamageEffect`))))
    (:`then_1`
      (`self.CheckDeath`))))

(event `/Game/Blueprints/Interfaces/BPI_LaserTrace.LaserHitEnd`
  (params (Laser :type "/Game/Blueprints/BP_Laser Object Reference"))
  (`self.RemoveDamageEffect`)
  (`self.ResetDamageEffect`))

(fn `(Temperory)MirroredLaserTrace`
  (params (ImpactNormal :type "Vector Structure") (Location :type "Vector Structure") (TraceEnd :type "Vector Structure") (TraceStart :type "Vector Structure"))
  (locals (IncidentVector :type "Vector Structure") (ReflectedVector :type "Vector Structure"))
  (set `local.IncidentVector` (- TraceEnd TraceStart))
  (bind _output_get (set `local.ReflectedVector` (- (`local.IncidentVector`) (* (* (`KismetMathLibrary.Dot_VectorVector` (`local.IncidentVector`) ImpactNormal) ImpactNormal) 2.0))))
  (bind _outhit (`KismetSystemLibrary.LineTraceSingle` :`Start` Location :`End` (* _output_get 1000.0) :`TraceChannel` "TraceTypeQuery1" :`DrawDebugType` "ForOneFrame" :`TraceColor` (struct :`G` 0.913099 :`B` 1.0 :`A` 1.0) :`TraceHitColor` (struct :`G` 0.913099 :`B` 1.0 :`A` 1.0))))

(fn `CheckDeath`
  (bind _result (`/Engine/EditorBlueprintResources/StandardMacros.DecrementFloat` (`self.Health`))
    (:`  `
      (if (<= _result 0.0)
        (`self.DestroyObject`)))))

(fn `DamageEffect`
  (`MeshComponent.SetOverlayMaterial` (`self.StaticMesh`) "/Game/LevelPrototyping/Materials/MI_FadedWhite.MI_FadedWhite"))

(fn `DestroyObject`
  (`self.K2_DestroyActor`))

(fn `RemoveDamageEffect`
  (`MeshComponent.SetOverlayMaterial` (`self.StaticMesh`) null))

(fn `UserConstructionScript`)